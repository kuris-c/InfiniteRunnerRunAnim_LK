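; BP_TileDefault_Liz is a tile actor that moves itself along the world X axis every frame.
; Tick calls UpdateTilesServer, which looks up all BP_Player actors each frame and scales the first one's TileSpeed by delta time.
; It prints the new X position and applies it to the root component with sweep, keeping Y and Z unchanged.
; Its own ForwardSpeed variable is unused.
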(event `self.ReceiveTick`
  (params (DeltaSeconds :type "Float (single-precision)"))
  (`self.UpdateTilesServer` DeltaSeconds))

(event `UpdateTilesServer`
  (params (DeltaSeconds :type "Float (double-precision)"))
  (bind (_x _y _z) (`KismetMathLibrary.BreakVector3f` (`SceneComponent.K2_GetComponentLocation` (`self.DefaultSceneRoot`))))
  (bind _outactors (`GameplayStatics.GetAllActorsOfClass` "/Game/Player/Blueprints/BP_Player.BP_Player_C"))
  (bind _returnvalue (+ (* DeltaSeconds (`/Game/Player/Blueprints/BP_Player.TileSpeed` (`|GetArrayItem` _outactors))) _x))
  (`KismetSystemLibrary.PrintString` (`KismetStringLibrary.Conv_DoubleToString` _returnvalue))
  (`SceneComponent.K2_SetWorldLocation` (`self.DefaultSceneRoot`) (`KismetMathLibrary.MakeVector` _returnvalue _y _z) true false))

(fn `UserConstructionScript`)