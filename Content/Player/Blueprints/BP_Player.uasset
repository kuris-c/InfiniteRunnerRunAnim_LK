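; BP_Player is the player Blueprint, handling basic movement with Enhanced Input.
; BeginPlay adds the player input mapping context, and the Movement action feeds its 2D value, flattened to Z=0, into AddMovementInput.
; Tick calls UpdateLocationServer and also runs the same capsule reposition, which keeps Y and Z while leaving X at its default, apparently pinning the player to a plane.
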(event `self.ReceiveBeginPlay`
  (`|ExecutionSequence`
    (:`then_1`
      ;[1 1 1] Player Movement
      (bind _asplayer_controller (cast `PlayerController` (`self.GetController`)))
      (`EnhancedInputSubsystemInterface.AddMappingContext` (pcsubsystem `EnhancedInputLocalPlayerSubsystem` _asplayer_controller) "/Game/Player/Input/Player_InputMapping.Player_InputMapping" 0 (struct)))))

(event `EnhancedInput|/Game/Player/Input/Movement`
  (params (ActionValue :type "Vector2D Structure") (ElapsedSeconds :type "Float (double-precision)") (TriggeredSeconds :type "Float (double-precision)") (InputAction :type "InputAction Object Reference" :default "/Game/Player/Input/Movement.Movement"))
  ;[1 1 1] Player Movement
  (:`Triggered`
    (`self.AddMovementInput` (`KismetMathLibrary.Conv_Vector2DToVector` ActionValue))))

(event `self.ReceiveTick`
  (params (DeltaSeconds :type "Float (single-precision)"))
  (bind (_returnvalue_x _returnvalue_y _returnvalue_z) (`KismetMathLibrary.BreakVector` (`SceneComponent.K2_GetComponentLocation` (`self.CapsuleComponent`))))
  (`self.UpdateLocationServer`)
  (`SceneComponent.K2_SetWorldLocation` (`self.CapsuleComponent`) (`KismetMathLibrary.MakeVector` 0.0 _returnvalue_y _returnvalue_z) false false :!label _label))

(event `UpdateLocationServer`
  (goto _label))

(fn `UserConstructionScript`)